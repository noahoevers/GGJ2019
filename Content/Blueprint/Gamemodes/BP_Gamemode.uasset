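; Game mode for a local split-screen cat-versus-mouse game that spawns the players and tracks a stress meter.
; BeginPlay calls CreatePlayersAndUI, which creates a player with a pawn per controller index.
; AdjustStressMeter caps stress at the maximum and then calls GameOver as a cat loss.
; It is unfinished: widget creation is unconnected, the cat branch and GameOver are empty, and below-maximum adjustments never add the amount.
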(event EventBeginPlay
  (CallFunction|CreatePlayersandUI (Variables|GameRelated|GetCurrentPlayers)))

(fn ConstructionScript)

(fn CreatePlayersandUI
  (params (AmountOfPlayers :type Integer))
  (for _index (range 0 (- AmountOfPlayers 1)) ; Starts at 1 because that is logical for currentplayers
    ;[1 1 1] Add all Ui and behaviour that all player need to have here
    (bind _returnvalue (Class|GameplayStatics|CreatePlayer _index))
    (if (Variables|UIRelated|GetIsCat?)
      _)))

(fn AdjustStressMeter
  (params (Adjust%20Amount :type Float%20%28single-precision%29))
  ;[1 1 1] Add stress meter value
  (if (>= (+ Adjust%20Amount (Variables|Default|GetStressMeterValue)) (Variables|Default|GetMaxStress))
    (Variables|Default|SetStressMeterValue (Variables|Default|GetMaxStress))
    (CallFunction|GameOver false)
    (else
      (bind _output_get (Variables|Default|SetStressMeterValue 0.0))
      (Development|PrintString (Utilities|String|Append "Stress meter level: " (Utilities|String|ToString(Float) _output_get)) true true "(R=0.000000,G=1.000000,B=0.031264,A=1.000000)"))))

(fn GameOver
  (params (DidCatWin? :type Boolean)))