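; BP_PickupObject is an interactable physical object that can be picked up and dropped, reacting to what it strikes.
; Pickup and drop effects toggle held state, hit ability and mesh collision ignoring with the interactor, and held objects refuse interaction.
; Box overlaps compare velocity to thresholds for a rate-limited impact sound and a hit.
; Hits send a break message for one weight class and can destroy the object.
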(event OnComponentBeginOverlap(Box)
  (params (OverlappedComponent :type Primitive%20Component%20Object%20Reference) (OtherActor :type Actor%20Object%20Reference) (OtherComp :type Primitive%20Component%20Object%20Reference) (OtherBodyIndex :type Integer) (bFromSweep :type Boolean) (SweepResult :type Hit%20Result%20Structure%20%28by%20ref%29))
  (bind _returnvalue (Transformation|GetVelocity))
  (bind _returnvalue_2 (Math|Vector|VectorLength _returnvalue))
  (Development|PrintString (Utilities|String|ToString(Float) _returnvalue_2))
  (if (>= _returnvalue_2 (Variables|Default|GetSpeedForSound))
    (CallFunction|OnSound OtherActor))
  (if (and (>= _returnvalue_2 (Variables|Default|GetSpeedForHit)) (Variables|Default|GetCanHit?))
    (CallFunction|OnHit OtherActor SweepResult)
    (if (Variables|Default|GetDestroyOnHit)
      (Actor|DestroyActor))))

(event EventBeginPlay
  (|CallParentFunction) ; This node is disabled and will not be called.\nDrag off pins to build functionality.
)

(event EventTick
  (params (DeltaSeconds :type Float%20%28single-precision%29))
  (|CallParentFunction DeltaSeconds) ; This node is disabled and will not be called.\nDrag off pins to build functionality.
)

(event EventPickUpEffects
  (params (Interactee :type BP%20Character%20Object%20Reference))
  (Collision|IgnoreActorwhenMoving (Variables|Default|GetStaticMesh) Interactee true)
  (Variables|Default|SetCanHit? false)
  (Variables|Default|SetBeingHeld? true))

(event EventDropEffects
  (params (Interactee :type BP%20Character%20Object%20Reference))
  (Collision|IgnoreActorwhenMoving (Variables|Default|GetStaticMesh) Interactee false)
  (Variables|Default|SetCanHit? true)
  (Variables|Default|SetBeingHeld? false))

(fn ConstructionScript
  (|CallParentFunction))

(fn OnSound
  (params (Actor :type Actor%20Object%20Reference))
  (bind _returnvalue (Utilities|Time|GetGameTimeinSeconds))
  (if (>= _returnvalue (+ (Variables|Default|GetTimeBetweenSounds) (Variables|Default|GetLastSoundTime)))
    (Variables|Default|SetLastSoundTime _returnvalue)
    (Audio|PlaySoundatLocation (Variables|Default|GetHitSound) (Transformation|GetActorLocation) "0, 0, 0" 1.0 1.0 0.0 0 0 0)))

(fn OnHit
  (params (Actor :type Actor%20Object%20Reference) (HitResult :type Hit%20Result%20Structure))
  (if (Utilities|Enum|Equal(Enum) (Variables|Default|GetWeight) "NewEnumerator1")
    (Class|BPIBreakable|OnBreak(Message) Actor)))

(fn CanInteract
  (params (Interactee :type BP%20Character%20Object%20Reference))
  (bind _caninteract_ (|CallParentFunction Interactee))
  (return (and _caninteract_ (not (Variables|Default|GetBeingHeld?)))))