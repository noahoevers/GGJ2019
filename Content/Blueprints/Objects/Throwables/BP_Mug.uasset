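; BP_Mug is a throwable mug that can be picked up, dropped and hit other actors.
; Pickup and drop effects toggle hit ability and ignoring the interactor during movement; BeingHeld, which blocks interaction, is set on drop and cleared on pickup.
; Overlaps above a speed threshold play a rate-limited sound.
; If also fast enough and hit-enabled, they send a break message for one Weight class and optionally destroy the mug.
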(event EventBeginPlay
  (|CallParentFunction) ; This node is disabled and will not be called.\nDrag off pins to build functionality.
)

(event Collision|EventActorBeginOverlap
  (params (OtherActor :type Actor%20Object%20Reference))
  (bind _returnvalue (Transformation|GetVelocity))
  (bind _returnvalue_2 (Math|Vector|VectorLength _returnvalue))
  (if (>= _returnvalue_2 (Variables|Default|GetSpeedForSound))
    (CallFunction|OnSound OtherActor)
    (if (and (>= _returnvalue_2 (Variables|Default|GetSpeedForHit)) (Variables|Default|GetCanHit?))
      (CallFunction|OnHit OtherActor)
      (if (Variables|Default|GetDestroyOnHit)
        (Actor|DestroyActor)))))

(event EventTick
  (params (DeltaSeconds :type Float%20%28single-precision%29))
  (|CallParentFunction DeltaSeconds) ; This node is disabled and will not be called.\nDrag off pins to build functionality.
)

(event EventPickUpEffects
  (params (Interactee :type BP%20Character%20Object%20Reference))
  (Collision|IgnoreActorwhenMoving (Variables|Default|GetStaticMesh) Interactee true)
  (Variables|Default|SetCanHit? false)
  (Variables|Default|SetBeingHeld? false))

(event EventDropEffects
  (params (Interactee :type BP%20Character%20Object%20Reference))
  (Collision|IgnoreActorwhenMoving (Variables|Default|GetStaticMesh) Interactee false)
  (Variables|Default|SetCanHit? true)
  (Variables|Default|SetBeingHeld? true))

(fn ConstructionScript
  (|CallParentFunction))

(fn OnSound
  (params (Actor :type Actor%20Object%20Reference))
  (bind _returnvalue (Utilities|Time|GetGameTimeinSeconds))
  (if (>= _returnvalue (+ (Variables|Default|GetTimeBetweenSounds) (Variables|Default|GetLastSoundTime)))
    (Variables|Default|SetLastSoundTime _returnvalue)
    (Audio|PlaySoundatLocation (Variables|Default|GetHitSound) (Transformation|GetActorLocation) "0, 0, 0" 1.0 1.0 0.0 0 0 0)))

(fn OnHit
  (params (Actor :type Actor%20Object%20Reference))
  (if (Utilities|Enum|Equal(Enum) (Variables|Default|GetWeight) "NewEnumerator1")
    (Class|BPIBreakable|OnBreak(Message) Actor)))

(fn CanInteract
  (params (Interactee :type BP%20Character%20Object%20Reference))
  (|CallParentFunction Interactee)
  (return (not (Variables|Default|GetBeingHeld?))))