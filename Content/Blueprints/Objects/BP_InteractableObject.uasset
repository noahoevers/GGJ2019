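; Interactable world object that players or items can dirty or break, and a sponge can clean, moving it between Normal, Dirty and Broken states.
; Player interaction runs a timeline once enough players join, updating their progress UI, and is allowed only while Normal.
; ChangeObjectState swaps mesh and material, then per-state handlers spawn effects, toggle a dynamic material's Dirty parameter and adjust the gamemode's stress meter.
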(event EventBeginPlay
  (|CallParentFunction)
  (CallFunction|ChangeObjectState "NewEnumerator0" true)
  (CallFunction|CreateMaterial))

(event Collision|EventActorBeginOverlap
  (params (OtherActor :type Actor%20Object%20Reference))
  (|CallParentFunction OtherActor) ; This node is disabled and will not be called.\nDrag off pins to build functionality.
)

(event EventTick
  (params (DeltaSeconds :type Float%20%28single-precision%29))
  (|CallParentFunction DeltaSeconds) ; This node is disabled and will not be called.\nDrag off pins to build functionality.
)

(event EventOnInteract
  (params (Interactee :type BP%20Character%20Object%20Reference))
  (Variables|Default|SetLastInteracteeRef Interactee)
  (Utilities|Array|Add (Variables|Default|GetCurrentPlayers) Interactee)
  (if (>= (Utilities|Array|Length (Variables|Default|GetCurrentPlayers)) (Variables|Default|GetPlayersNeeded))
    (Components|Timeline|SetPlayRate (Variables|Default|GetInteractTimeline) (/ 1.0 (Variables|Default|GetTimeToInteract)))
    (bind _percentagedone (Timeline|InteractTimeline PlayFromStart)
      (:Update
        (for _array_element (Variables|Default|GetCurrentPlayers)
          (Default|ChangeInteractPercentage (Variables|/Game/Blueprints/Characters/BP_Character.BP_Character_C|GetInteractingUI _array_element) _percentagedone)))
      (:Finished
        (CallFunction|OnFinishInteract (Variables|Default|GetCurrentPlayers))))))

(event EventOnStopInteract
  (params (Interactee :type BP%20Character%20Object%20Reference))
  (Default|ChangeInteractPercentage (Variables|/Game/Blueprints/Characters/BP_Character.BP_Character_C|GetInteractingUI Interactee) 0.0)
  (Utilities|Array|RemoveItem (Variables|Default|GetCurrentPlayers) Interactee)
  (if (<= (Utilities|Array|Length (Variables|Default|GetCurrentPlayers)) (Variables|Default|GetPlayersNeeded))
    (bind _percentagedone (Timeline|InteractTimeline Stop)
      (:Update
        (for _array_element (Variables|Default|GetCurrentPlayers)
          (Default|ChangeInteractPercentage (Variables|/Game/Blueprints/Characters/BP_Character.BP_Character_C|GetInteractingUI _array_element) _percentagedone)))
      (:Finished
        (CallFunction|OnFinishInteract (Variables|Default|GetCurrentPlayers))))))

(event EventOnClean
  (params (BP_Sponge :type BP%20Sponge%20Object%20Reference))
  (CallFunction|ChangeObjectState "NewEnumerator0" false BP_Sponge))

(event EventOnBreak
  (if (Variables|ObjectSpecifications|GetCanBeDestroyedByItems)
    (CallFunction|ChangeObjectState "NewEnumerator2" false)))

(event EventOnDirty
  (if (Variables|ObjectSpecifications|GetCanBeDirtyByItems)
    (CallFunction|ChangeObjectState "NewEnumerator1" false)))

(fn ConstructionScript
  (|CallParentFunction))

(fn OnFinishInteract
  (params (Characters :type Array%20of%20BP%20Character%20Object%20References))
  (if (Variables|ObjectSpecifications|GetCanBeDestroyedByInteraction)
    (Development|PrintString "You shit a brick an object!" true true "(R=1.000000,G=0.231851,B=0.152145,A=1.000000)" 5.0)
    (CallFunction|ChangeObjectState "NewEnumerator2" false)
    (elif (Variables|ObjectSpecifications|GetDirtyByInteraction)
      (Development|PrintString "You shit on an object!" true true "(R=1.000000,G=0.231851,B=0.152145,A=1.000000)" 5.0)
      (CallFunction|ChangeObjectState "NewEnumerator1" false))))

(fn ChangeObjectState
  (params (ObjectState :type E_ObjectState%20Enum :default "NewEnumerator0") (Initial :type Boolean) (Target :type BP%20Sponge%20Object%20Reference))
  (bind _dynamicnormalmaterial (Variables|Default|GetDynamicNormalMaterial))
  (LocalVariables|SetPreviousObjectState (Variables|Default|GetObjectState))
  (if (Utilities|Enum|NotEqual(Enum) (Variables|Default|GetObjectState) "NewEnumerator2")
    (bind _output_get (Variables|Default|SetObjectState ObjectState))
    (Components|StaticMesh|SetStaticMesh (Variables|Default|GetStaticMesh) (Utilities|Select :Index _output_get :NewEnumerator0 (Variables|Default|GetNormalMesh) :NewEnumerator1 (Variables|Default|GetDirtyMesh) :NewEnumerator2 (Variables|Default|GetBrokenMesh)))
    (Rendering|Material|SetMaterial (Variables|Default|GetStaticMesh) (Variables|Default|GetMaterialID) (Utilities|Select :Index _output_get :NewEnumerator0 _dynamicnormalmaterial :NewEnumerator1 _dynamicnormalmaterial :NewEnumerator2 (Variables|Default|GetBrokenMaterial)))
    (switch Utilities|FlowControl|Switch|SwitchonE_ObjectState (Variables|Default|GetObjectState)
      (:NewEnumerator0
        (CallFunction|SwitchtoNormal (LocalVariables|GetPreviousObjectState) Initial Target))
      (:NewEnumerator1
        (CallFunction|SwitchtoDirty (LocalVariables|GetPreviousObjectState)))
      (:NewEnumerator2
        (CallFunction|SwitchtoDestroy (LocalVariables|GetPreviousObjectState))))))

(fn AdjustStress
  (params (Change :type Float%20%28single-precision%29))
  (bind _asbp_main_gamemode (Utilities|Casting|CastToBP_MainGamemode (Game|GetGameMode))
    (:then
      (Default|AdjustStressMeter _asbp_main_gamemode Change)
      (Development|PrintString (Utilities|String|ToString(Float) Change)))
    (:CastFailed
      (Development|PrintString "ded"))))

(fn SwitchtoNormal
  (params (OldState :type E_ObjectState%20Enum :default "NewEnumerator0") (Initial :type Boolean) (Target :type BP%20Sponge%20Object%20Reference))
  (if Initial
    _
    (else
      (Rendering|Material|SetScalarParameterValue (Variables|Default|GetDynamicNormalMaterial) "Dirty" 0.0 :!class /Script/Engine.MaterialInstanceDynamic)))
  (switch Utilities|FlowControl|Switch|SwitchonE_ObjectState OldState
    (:NewEnumerator1
      (CallFunction|AdjustStress (* (Variables|Default|GetScoreForDirty) -1.0))
      (Default|UseCharge Target)
      (Audio|PlaySoundatLocation "/Game/Audio/Scrub/Scrub_Cue.Scrub_Cue" (Transformation|GetActorLocation) "0, 0, 0" 1.0 1.0 0.0 0 0 0)
      (Effects|SpawnEmitterAttached "/Game/Art/VFX/VFX_files/cleansmokePFX.cleansmokePFX" (Variables|Default|GetStaticMesh) "None" (Transformation|GetWorldLocation (Variables|Default|GetStaticMesh)) "0, 0, 0" "10.000000,10.000000,10.000000" "KeepWorldPosition"))
    (:NewEnumerator2
      (CallFunction|AdjustStress (* (Variables|Default|GetScoreForDestroy) -1.0)))))

(fn SwitchtoDirty
  (params (OldState :type E_ObjectState%20Enum :default "NewEnumerator0"))
  (Effects|SpawnEmitterAttached "/Game/Art/VFX/VFX_files/dirtsmokePFX.dirtsmokePFX" (Variables|Default|GetStaticMesh) "None" (Transformation|GetWorldLocation (Variables|Default|GetStaticMesh)) "0, 0, 0" "10.000000,10.000000,10.000000" "KeepWorldPosition")
  (Rendering|Material|SetScalarParameterValue (Variables|Default|GetDynamicNormalMaterial) "Dirty" 1.0 :!class /Script/Engine.MaterialInstanceDynamic)
  (switch Utilities|FlowControl|Switch|SwitchonE_ObjectState OldState
    (:NewEnumerator0
      (CallFunction|AdjustStress (* (Variables|Default|GetScoreForDirty) 1.0)))))

(fn SwitchtoDestroy
  (params (OldState :type E_ObjectState%20Enum :default "NewEnumerator0"))
  (Effects|SpawnEmitterAttached "/Game/Art/VFX/VFX_files/breaksmokePFX.breaksmokePFX" (Variables|Default|GetStaticMesh) "None" (Transformation|GetWorldLocation (Variables|Default|GetStaticMesh)) "0, 0, 0" "10.000000,10.000000,10.000000" "KeepWorldPosition")
  (switch Utilities|FlowControl|Switch|SwitchonE_ObjectState OldState
    (:NewEnumerator0
      (CallFunction|AdjustStress (* (Variables|Default|GetScoreForDestroy) 1.0)))
    (:NewEnumerator1
      (CallFunction|AdjustStress (* (- (Variables|Default|GetScoreForDestroy) (Variables|Default|GetScoreForDirty)) 1.0)))))

(fn CreateMaterial
  (bind _returnvalue (Rendering|Material|CreateDynamicMaterialInstance (Rendering|Material|GetMaterial (Variables|Default|GetStaticMesh) 0) "None" :!class /Script/Engine.KismetMaterialLibrary))
  (Variables|Default|SetDynamicNormalMaterial _returnvalue))

(fn CanInteract
  (params (Interactee :type BP%20Character%20Object%20Reference))
  (bind _caninteract_ (|CallParentFunction Interactee))
  (return (and _caninteract_ (not (or (Utilities|Enum|Equal(Enum) (Variables|Default|GetObjectState) "NewEnumerator2") (Utilities|Enum|Equal(Enum) (Variables|Default|GetObjectState) "NewEnumerator1"))))))