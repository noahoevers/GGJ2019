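; BP_PooStain is a cleanable stain actor that affects the game's stress meter.
; On BeginPlay it adds its StressValue to the meter through BP_MainGamemode.
; Its OnClean event subtracts the same amount from the meter and destroys the actor.
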(event EventBeginPlay
  (bind _asbp_main_gamemode (Utilities|Casting|CastToBP_MainGamemode (Game|GetGameMode)))
  (Default|AdjustStressMeter _asbp_main_gamemode (Variables|Default|GetStressValue)))

(event Collision|EventActorBeginOverlap
  (params (OtherActor :type Actor%20Object%20Reference)))

(event EventTick
  (params (DeltaSeconds :type Float%20%28single-precision%29)))

(event EventOnClean
  (bind _asbp_main_gamemode (Utilities|Casting|CastToBP_MainGamemode (Game|GetGameMode)))
  (Default|AdjustStressMeter _asbp_main_gamemode (* (Variables|Default|GetStressValue) -1.0))
  (Actor|DestroyActor))

(fn ConstructionScript)