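; BP_LITterbox is a litterbox object that keeps a BP_Poo actor available in the level.
; It spawns one at its PooSpawn component on BeginPlay and binds to that actor's OnDestroyed event.
; When the poo is destroyed, a one-shot timer of PooRespawn length calls SpawnPoo again, repeating the cycle.
; Each spawn also prints the new actor's display name.
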(event Custom|SpawnPoo
  (bind _returnvalue (Game|SpawnActorfromClass "/Game/Blueprints/Objects/DirtyObjects/BP_Poo.BP_Poo_C" (Math|Transform|MakeTransform (Transformation|GetWorldLocation (Variables|Default|GetPooSpawn)) "0, 0, 0" "1,1,1") "AdjustIfPossibleButAlwaysSpawn" 0 0))
  (Game|BindEventtoOnDestroyed _returnvalue (delegate Custom|OnPooDestroy))
  (Development|PrintString (Utilities|GetDisplayName _returnvalue)))

(event Custom|OnPooDestroy
  (params (DestroyedActor :type Actor%20Object%20Reference))
  (Utilities|Time|SetTimerbyEvent (delegate Custom|SpawnPoo) (Variables|Default|GetPooRespawn)))

(event EventBeginPlay
  (CallFunction|SpawnPoo))

(fn ConstructionScript)